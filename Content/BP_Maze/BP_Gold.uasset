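; BP_Gold is a gold pickup for the maze game, worth a random amount from 1 to 99.
; The construction script rolls the value and uses a CreateMesh macro to add up to three randomly offset and scaled meshes, so richer piles look bigger.
; BeginPlay caches the MazeGamemode and shows the value on a text render.
; Interact adds the value to the game mode's PlayerGold and destroys the actor.
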(event `self.ReceiveBeginPlay`
  (bind _asmaze_gamemode (cast `/Game/BP_Maze/MazeGamemode` (`GameplayStatics.GetGameMode`)))
  (set `self.As Gamemode` _asmaze_gamemode)
  (`TextRenderComponent.K2_SetText` (`self.TextRender`) (`KismetTextLibrary.Conv_IntToText` (`self.Gold`))))

(event `/Game/BP_Maze/MazeInterface.Interact`
  (bind _as_gamemode (`self.As Gamemode`))
  (set `/Game/BP_Maze/MazeGamemode.PlayerGold` (+ (`/Game/BP_Maze/MazeGamemode.PlayerGold` _as_gamemode) (`self.Gold`)) _as_gamemode)
  (`self.K2_DestroyActor`))

(fn `UserConstructionScript`
  (bind _gold (`self.Gold`))
  (set `self.Gold` (`KismetMathLibrary.RandomIntegerInRange` 1 99))
  (`self.CreateMesh` (>= _gold 76)
    (:`Out`
      _)
    (:`False`
      _))
  (`self.CreateMesh` (>= _gold 26)
    (:`Out`
      _)
    (:`False`
      _))
  (`self.CreateMesh` (>= _gold 1)))