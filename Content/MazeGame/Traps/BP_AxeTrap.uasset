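; BP_AxeTrap is a maze-game trap that swings an axe and damages the player character.
; BeginPlay caches the third-person player character, and both trigger overlaps respond only to that actor.
; Entering the Activision volume plays the Axes timeline, whose track is scaled to drive the axe's relative pitch.
; Entering DamageBox applies a fixed health penalty through the character's HealthUpdate, independently of whether the axe is moving.
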(event `self.ReceiveBeginPlay`
  (bind _asbp_third_person_character (cast `/Game/ThirdPerson/Blueprints/BP_ThirdPersonCharacter` (`GameplayStatics.GetPlayerCharacter` 0)))
  (set `self.As BP Third Person Character` _asbp_third_person_character))

(event `self.DamageBox.OnComponentBeginOverlap`
  (params (OverlappedComponent :type "PrimitiveComponent Object Reference") (OtherActor :type "Actor Object Reference") (OtherComp :type "PrimitiveComponent Object Reference") (OtherBodyIndex :type Integer) (bFromSweep :type Boolean) (SweepResult :type "HitResult Structure (by ref)"))
  (bind _as_bp_third_person_character (`self.As BP Third Person Character`))
  (if (== OtherActor _as_bp_third_person_character)
    (`/Game/ThirdPerson/Blueprints/BP_ThirdPersonCharacter.HealthUpdate` _as_bp_third_person_character -15.0)))

(event `self.Activision.OnComponentBeginOverlap`
  (params (OverlappedComponent :type "PrimitiveComponent Object Reference") (OtherActor :type "Actor Object Reference") (OtherComp :type "PrimitiveComponent Object Reference") (OtherBodyIndex :type Integer) (bFromSweep :type Boolean) (SweepResult :type "HitResult Structure (by ref)"))
  (if (== OtherActor (`self.As BP Third Person Character`))
    (bind (_direction _newtrack_0) (`Timeline|Axes`)
      (:`Update`
        (`SceneComponent.K2_SetRelativeRotation` (`self.Axe`) (`KismetMathLibrary.MakeRotator` 0.0 (* _newtrack_0 330.0)) false false)))))

(fn `UserConstructionScript`)